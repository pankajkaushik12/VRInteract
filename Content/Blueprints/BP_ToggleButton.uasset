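; BP_ToggleButton is a placeable button that toggles the visibility of a referenced object, ObjectToToggle.
; On BeginPlay it spawns a BP_Button at its own transform and binds to that button's pressed and released events, or prints a warning if no object is set.
; Both events send the ToggleVisibility message to the object, so visibility flips on press and again on release.
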(event `self.ReceiveBeginPlay`
  (`/Engine/EditorBlueprintResources/StandardMacros.IsValid` (`self.ObjectToToggle`)
    (:`Is Valid`
      (bind _returnvalue (`|SpawnActorFromClass` "/Game/Blueprints/BP_Button.BP_Button_C" (`self.GetTransform`) "Undefined" "MultiplyWithRoot" null null))
      (add `/Game/Blueprints/BP_Button.OnButtonPressed` _returnvalue (delegate `OnButtonPressed_Event`))
      (add `/Game/Blueprints/BP_Button.OnButtonReleased` _returnvalue (delegate `OnButtonReleased_Event`)))
    (:`Is Not Valid`
      (`KismetSystemLibrary.PrintString` "Object is not set."))))

(event `OnButtonReleased_Event`
  (params (Button :type "/Game/Blueprints/BP_Button Object Reference"))
  (message `/Game/Blueprints/BPI_ActorProperty.ToggleVisibility` (`self.ObjectToToggle`)))

(event `OnButtonPressed_Event`
  (params (Button :type "/Game/Blueprints/BP_Button Object Reference"))
  (message `/Game/Blueprints/BPI_ActorProperty.ToggleVisibility` (`self.ObjectToToggle`)))

(fn `UserConstructionScript`)