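; BP_Button is an animated button driven by number keys, with input enabled on BeginPlay.
; Key 3 passes a DoOnce to play or reverse a timeline, depending on IsHandOverlapping.
; Each forward update moves the Scene component, flips that flag and resets the DoOnce after a delay.
; Keys 4 and 5 fire pressed and released calls, while key 2 toggles a referenced object's visibility.
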(event `self.ReceiveBeginPlay`
  (`self.EnableInput` (`GameplayStatics.GetPlayerController` 0)))

(event `Key|Three`
  (params (Key :type "Key Structure"))
  (:`Pressed`
    (`/Engine/EditorBlueprintResources/StandardMacros.DoOnce` false :!label _label
      (:`Completed`
        (if (`self.IsHandOverlapping`)
          (bind (_direction _positionz) (`Timeline|ButtonAnimTimeline` :!label _label_2)
            (:`Update`
              (`SceneComponent.K2_SetRelativeLocation` (`self.Scene`) _positionz false false)
              (bind _output_get (set `self.IsHandOverlapping` (not (`self.IsHandOverlapping`))))
              (`KismetSystemLibrary.PrintString` (`KismetStringLibrary.Conv_BoolToString` _output_get))
              (`KismetSystemLibrary.Delay` 0.5)
              (goto _label :!via `Reset`)))
          (else
            (goto _label_2 :!via `Reverse`)))))))

(event `Key|Four`
  (params (Key :type "Key Structure"))
  (:`Pressed`
    (`self.OnButtonPressed` self)))

(event `Key|Five`
  (params (Key :type "Key Structure"))
  (:`Pressed`
    (`self.OnButtonReleased` self)))

(event `Key|Two`
  (params (Key :type "Key Structure"))
  (bind _objecttotoggle (`self.ObjectToToggle`))
  (:`Pressed`
    (`/Engine/EditorBlueprintResources/StandardMacros.IsValid` _objecttotoggle
      (:`Is Valid`
        (message `/Game/Blueprints/BPI_ActorProperty.ToggleVisibility` _objecttotoggle))
      (:`Is Not Valid`
        (`KismetSystemLibrary.PrintString` "Object is not set.")))))

(fn `UserConstructionScript`)