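; BP_AnimManager is an actor that provides buttons to start and stop animations, allowing one at a time.
; On BeginPlay it spawns a BP_Button for each Animations entry in a row along Y and binds to its press and release events.
; Pressing sends a start message to the entry at the matching index unless one is running.
; Releasing while one runs clears the flag and sends stop to that button's entry.
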(event `self.ReceiveBeginPlay`
  (bind _returnvalue (`self.GetTransform`))
  (for _index (range (`KismetArrayLibrary.Array_Length` (`self.Animations`)))
    (bind _returnvalue_2 (`|SpawnActorFromClass` "/Game/Blueprints/BP_Button.BP_Button_C" (`KismetMathLibrary.MakeTransform` (`KismetMathLibrary.MakeVector` (.x (.location _returnvalue)) (+ (* _index 100) (.y (.location _returnvalue))) (.z (.location _returnvalue))) (.rotation _returnvalue) (.scale _returnvalue)) "Undefined" "MultiplyWithRoot" null null))
    (`KismetArrayLibrary.Array_Add` (`self.Buttons`) _returnvalue_2)
    (add `/Game/Blueprints/BP_Button.OnButtonPressed` _returnvalue_2 (delegate `OnButtonPressed_Event`))
    (add `/Game/Blueprints/BP_Button.OnButtonReleased` _returnvalue_2 (delegate `OnButtonReleased_Event`))))

(event `OnButtonPressed_Event`
  (params (Button :type "/Game/Blueprints/BP_Button Object Reference"))
  (if (`self.IsAnimationRunning`)
    (`KismetSystemLibrary.PrintString` "An animation is already playing. Stop it to play another animation.")
    (else
      (set `self.IsAnimationRunning` true)
      (message `/Game/Blueprints/BPI_Animations.StartAnimation` (`|GetArrayItem` (`self.Animations`) (`KismetArrayLibrary.Array_Find` (`self.Buttons`) Button))))))

(event `OnButtonReleased_Event`
  (params (Button :type "/Game/Blueprints/BP_Button Object Reference"))
  (if (`self.IsAnimationRunning`)
    (set `self.IsAnimationRunning` false)
    (message `/Game/Blueprints/BPI_Animations.StopAnimation` (`|GetArrayItem` (`self.Animations`) (`KismetArrayLibrary.Array_Find` (`self.Buttons`) Button)))))

(fn `UserConstructionScript`)